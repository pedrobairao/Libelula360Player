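; BP_Interactive_Menu is an interactive actor that represents a project and transports the player into it.
; SetUp stores the project ID and name, applies the anchor material to its mesh, sets the label text and positions the actor.
; On Activate it plays a fade-out level sequence, waits briefly, writes the project ID to the AppContext game instance, then opens the Project level.
; EditDoor is an empty stub.
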(event `self.Activate`
  ;[1 1 1] Activate - Transport
  (`self.Transition`)
  (`KismetSystemLibrary.Delay` 2.0)
  (bind _asapp_context (cast `/Game/SaveSettings/AppContext` (`GameplayStatics.GetGameInstance`)))
  (set `/Game/SaveSettings/AppContext.CurrentProjectID` (`KismetStringLibrary.Conv_NameToString` (`self.Project`)) _asapp_context)
  (`GameplayStatics.OpenLevel` "Project"))

(fn `EditDoor`)

(fn `SetUp`
  (params (AnchorMaterial :type "MaterialInterface Object Reference") (ProjectID :type Name) (ProjectName :type String) (Transform :type "Transform Structure"))
  (set `self.Project` ProjectID)
  (bind _output_get (set `self.ProjectName` ProjectName))
  (bind _output_get_2 (set `self.AnchorMaterial` AnchorMaterial))
  (`PrimitiveComponent.SetMaterial` (`self.StaticMesh`) 0 _output_get_2)
  (`TextRenderComponent.K2_SetText` (`self.Label`) (`KismetTextLibrary.Conv_StringToText` _output_get))
  (bind _output_get_3 (set `self.Transform` Transform))
  (`self.K2_SetActorTransform` _output_get_3)
  (`self.Update`))

(fn `Transition`
  (bind _outactor (`LevelSequencePlayer.CreateLevelSequencePlayer` "/Game/Assets/Sequences/FadeOut_Sequence/FadeOut_SequenceMaster.FadeOut_SequenceMaster"))
  (`MovieSceneSequencePlayer.Play` (`LevelSequenceActor.SequencePlayer` _outactor)))

(fn `UserConstructionScript`
  (`parent.UserConstructionScript`))