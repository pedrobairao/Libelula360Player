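; Player camera pawn for VR-style gaze interaction, with mouse head-look scaled by the game instance's sensitivity and an M key return to the menu.
; Each tick traces forward from the camera; newly focusing a BP_InteractiveBase starts a timer and cursor progress bar.
; When the timer ends the object activates; looking away cancels it.
; Helper functions fade the camera and switch edit and preview modes, toggling the VR cursor.
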(event `self.ReceiveBeginPlay`
  ;[1 1 1] Begin Play
  (bind _asapp_context (cast `/Game/SaveSettings/AppContext` (`GameplayStatics.GetGameInstance`)))
  (bind _output_get (set `/Game/SaveSettings/AppContext.isEditMode` false _asapp_context))
  (bind _output_get_2 (set `/Game/SaveSettings/AppContext.PreviewEdit` false _asapp_context))
  (set `self.isEditMode` _output_get)
  (set `self.PreviewEdit` _output_get_2)
  (set `self.HeadMovement Sensitivity` (`/Game/SaveSettings/AppContext.Sensitivity` _asapp_context))
  (bind _returnvalue (`|CreateWidget` "/Game/UI/HUD/WBP_VR_Cursor.WBP_VR_Cursor_C" (`GameplayStatics.GetPlayerController` 0)))
  (bind _output_get_3 (set `self.Timer W Ref` _returnvalue))
  (`UserWidget.AddToViewport` _output_get_3 0))

(event `Key|M`
  (params (Key :type "Key Structure"))
  ;[1 1 1] Back to Menu
  (:`Pressed`
    (`GameplayStatics.OpenLevel` "ImersiveMenu")))

(event `self.ReceiveTick`
  (params (DeltaSeconds :type "Float (single-precision)"))
  ;[1 1 1] Gaze
  (`self.Time BasicGaze`))

(event `InputAxisKey|MouseX`
  (params (AxisValue :type "Float (single-precision)"))
  ;[1 1 1] Editor Head Movement
  (`self.AddControllerYawInput` (* (* AxisValue (`GameplayStatics.GetWorldDeltaSeconds`)) (`self.HeadMovement Sensitivity`))))

(event `InputAxisKey|MouseY`
  (params (AxisValue :type "Float (single-precision)"))
  ;[1 1 1] Editor Head Movement
  (`self.AddControllerPitchInput` (* (* (* AxisValue (`GameplayStatics.GetWorldDeltaSeconds`)) (`self.HeadMovement Sensitivity`)) -1.0)))

(fn `BasicGaze`
  (bind (_bblockinghit _binitialoverlap _time _distance _location _impactpoint _normal _impactnormal _physmat _hitactor) (`GameplayStatics.BreakHitResult` (`self.LineTraceForward`)))
  (if _bblockinghit
    (bind _asbp_interactive_base (cast `/Game/Blueprints/BP_InteractiveBase` _hitactor))
    (set `self.Interactive Object` _asbp_interactive_base)
    (if (not (== (`self.Interactive Object`) (`self.Focused Object`)))
      (set `self.Focused Object` (`self.Interactive Object`))
      (`self.Interact`))
    (else
      (set `self.Interactive Object` null)
      (set `self.Focused Object` null))))

(fn `Interact`
  (bind _interactive_object (`self.Interactive Object`))
  (`/Engine/EditorBlueprintResources/StandardMacros.IsValid` _interactive_object
    (:`Is Valid`
      (`/Game/UI/HUD/WBP_VR_Cursor.Hide Timer Bar` (`self.Timer W Ref`))
      (`/Game/Blueprints/BP_InteractiveBase.Activate` _interactive_object))))

(fn `LineTraceForward`
  (returns (OutHit :type "HitResult Structure"))
  (bind _camera (`self.Camera`))
  (bind _returnvalue (`SceneComponent.K2_GetComponentLocation` _camera))
  (bind _outhit (`KismetSystemLibrary.LineTraceSingle` _returnvalue (+ _returnvalue (* (`KismetMathLibrary.GetForwardVector` (`SceneComponent.K2_GetComponentRotation` _camera)) 20000.0)) "TraceTypeQuery1"))
  (return _outhit))

(fn `SetEditMode`
  (set `self.isEditMode` true)
  (`/Game/UI/HUD/WBP_VR_Cursor.Hide Vr Cursor` (`self.Timer W Ref`)))

(fn `SetPreviewMode`
  (bind _timer_w_ref (`self.Timer W Ref`))
  (set `self.isEditMode` false)
  (`UserWidget.AddToViewport` _timer_w_ref 0)
  (`/Game/UI/HUD/WBP_VR_Cursor.Display VR Cursor` _timer_w_ref))

(fn `Time BasicGaze`
  (bind (_bblockinghit _binitialoverlap _time _distance _location _impactpoint _normal _impactnormal _physmat _hitactor) (`GameplayStatics.BreakHitResult` (`self.LineTraceForward`)))
  (if _bblockinghit
    (set `self.Gaze impact Point` _impactpoint)
    (bind _asbp_interactive_base (cast `/Game/Blueprints/BP_InteractiveBase` _hitactor)
      (:`then`
        (set `self.Interactive Object` _asbp_interactive_base)
        (if (not (== (`self.Interactive Object`) (`self.Focused Object`)))
          (set `self.Focused Object` (`self.Interactive Object`))
          (`KismetSystemLibrary.K2_ClearAndInvalidateTimerHandle` (`self.Focus Timer`))
          (bind _returnvalue (`KismetSystemLibrary.K2_SetTimer` null "Interact" (`self.Timer Lenght`)))
          (set `self.Focus Timer` _returnvalue)
          (`/Game/UI/HUD/WBP_VR_Cursor.Display Timer Bar` (`self.Timer W Ref`))))
      (:`CastFailed`
        (set `self.Interactive Object` null :!label _label)
        (set `self.Focused Object` null)
        (`KismetSystemLibrary.K2_ClearAndInvalidateTimerHandle` (`self.Focus Timer`))
        (`/Game/UI/HUD/WBP_VR_Cursor.Hide Timer Bar` (`self.Timer W Ref`))))
    (else
      (goto _label))))

(fn `Transition`
  (`PlayerCameraManager.StartCameraFade` :`self` (`GameplayStatics.GetPlayerCameraManager` 0) :`ToAlpha` 1.0 :`Duration` 2.0 :`bHoldWhenFinished` true))

(fn `UserConstructionScript`)