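; Interactive hotspot actor: a configurable anchor mesh that runs an assigned action when activated.
; SetUp applies mesh, transform and either a given material or one loaded from an image file, then packs the settings into a HotspotStruct.
; It hides flagged hotspots in game unless the AppContext game instance is in edit mode.
; Activate passes the transform and action struct to ActionFunction; EditHotspot is an empty stub.
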(event `self.Activate`
  ;[1 1 1] Activate
  (`/Game/Blueprints/BP_ActionFunction.DoAction` (`self.ActionFunction`) (`self.Transform`) (`self.ActionStruct`)))

(fn `EditHotspot`)

(fn `SetAction`
  (params (Action :type "/Game/SaveSettings/Action_Struct Structure"))
  (set `self.ActionStruct` Action))

(fn `SetUp`
  (params (AnchorMaterial :type "MaterialInterface Object Reference") (AnchorMesh :type "StaticMesh Object Reference") (NewTransform :type "Transform Structure (by ref)") (Hide :type Boolean) (ID :type Name) (Action :type "/Game/SaveSettings/Action_Struct Structure") (isFile :type Boolean) (Filename :type String))
  (bind _staticmesh (`self.StaticMesh`))
  (set `self.Anchor_ID` ID)
  (set `self.ActionStruct` Action)
  (bind _output_get (set `self.AnchorMesh` AnchorMesh))
  (`StaticMeshComponent.SetStaticMesh` (`self.StaticMesh`) _output_get)
  (bind _output_get_2 (set `self.isFile` isFile))
  (bind _output_get_3 (set `self.Filename` Filename))
  (if _output_get_2
    (bind _materialinstance (`/Game/Blueprints/LoadAssets.LoadImage` _output_get_3))
    (bind _output_get_4 (set `self.AnchorMaterial` _materialinstance))
    (`PrimitiveComponent.SetMaterial` _staticmesh 0 _output_get_4)
    (else
      (bind _output_get_5 (set `self.AnchorMaterial` AnchorMaterial))
      (`PrimitiveComponent.SetMaterial` _staticmesh 0 _output_get_5)))
  (bind _output_get_6 (set `self.Hide` Hide))
  (bind _asapp_context (cast `/Game/SaveSettings/AppContext` (`GameplayStatics.GetGameInstance`)))
  (`self.SetActorHiddenInGame` (and (not (`/Game/SaveSettings/AppContext.isEditMode` _asapp_context)) _output_get_6))
  (bind _output_get_7 (set `self.Transform` NewTransform))
  (`self.K2_SetActorTransform` _output_get_7)
  (set `self.Hotspot_Struct` (make `/Game/SaveSettings/Hotspot_Struct` (`self.AnchorMaterial`) (`self.AnchorMesh`) (`self.Transform`) (`self.Hide`) (`self.Anchor_ID`) (`self.ActionStruct`) (`self.isFile`) (`self.Filename`))))

(fn `UserConstructionScript`
  (`parent.UserConstructionScript`))