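; LoadAssets loads image and video files from disk at runtime, resolving names against the Path held by the AppContext game instance.
; LoadImage imports a file as a texture and feeds it into a new dynamic instance of 360_Mat_Inst, returning both with the texture size.
; LoadVideo points a shared media source at the file, opens and plays it on the player, and returns the video material and media objects.
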(fn `LoadImage`
  (params (File :type String))
  (returns (MaterialInstance :type "MaterialInstanceDynamic Object Reference") (Texture2d :type "Texture2D Object Reference") (sizeX :type Integer) (sizeY :type Integer))
  (locals (Path :type String :default "C:\\Users\\Pedrp\\Documents\\Unreal Projects\\Libelula360Creator\\Content\\Images\\") (Mat :type "Material Object Reference" :default "Material'/Game/Assets/Backgrounds/360_Mat.360_Mat'") (Mat_Inst :type "MaterialInstance Object Reference" :default "MaterialInstanceConstant'/Game/Assets/Backgrounds/360_Mat_Inst.360_Mat_Inst'"))
  (bind _asapp_context (cast `/Game/SaveSettings/AppContext` (`GameplayStatics.GetGameInstance` null)))
  (bind _returnvalue (`KismetRenderingLibrary.ImportFileAsTexture2D` null (`KismetStringLibrary.Concat_StrStr` (`/Game/SaveSettings/AppContext.Path` _asapp_context) File)))
  (bind _returnvalue_2 (`KismetMaterialLibrary.CreateDynamicMaterialInstance` null "/Game/Assets/Backgrounds/360_Mat_Inst.360_Mat_Inst" (`KismetStringLibrary.Conv_StringToName` File)))
  (`MaterialInstanceDynamic.SetTextureParameterValue` _returnvalue_2 "TextureParam" _returnvalue)
  (return _returnvalue_2 _returnvalue (`Texture2D.Blueprint_GetSizeX` _returnvalue) (`Texture2D.Blueprint_GetSizeY` _returnvalue)))

(fn `LoadVideo`
  (params (InputPin :type String))
  (returns (Material :type "MaterialInterface Object Reference") (MediaPlayer :type "MediaPlayer Object Reference") (MediaSource :type "MediaSource Object Reference") (opened :type Boolean))
  (locals (Player :type "MediaPlayer Object Reference" :default "MediaPlayer'/Game/Assets/Backgrounds/Movies/Load_MediaPlayer.Load_MediaPlayer'") (Source :type "FileMediaSource Object Reference" :default "FileMediaSource'/Game/Assets/Backgrounds/Movies/Load_Media.Load_Media'") (VideoMaterial :type "MaterialInterface Object Reference" :default "Material'/Game/Assets/Backgrounds/Movies/Load_MediaPlayer_Video_Mat.Load_MediaPlayer_Video_Mat'"))
  (bind _player (`local.Player`))
  (bind _source (`local.Source`))
  (bind _asapp_context (cast `/Game/SaveSettings/AppContext` (`GameplayStatics.GetGameInstance` null)))
  (`FileMediaSource.SetFilePath` _source (`KismetStringLibrary.Concat_StrStr` (`/Game/SaveSettings/AppContext.Path` _asapp_context) InputPin))
  (bind _returnvalue (`MediaPlayer.OpenSource` _player _source))
  (`MediaPlayer.Play` _player)
  (return (`local.VideoMaterial`) _player _source _returnvalue))